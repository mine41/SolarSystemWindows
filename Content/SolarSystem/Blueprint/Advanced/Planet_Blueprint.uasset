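; Planet actor for a solar system scene that circles a target actor on a flat orbit while spinning on its own axis.
; BeginPlay optionally spawns a scaled Orbit_Blueprint at the target as the orbit line.
; Tick accumulates a delta-time-scaled, direction-signed angle for RotateAroundPoint, which sets position from the target's current location.
; Self-spin is a fixed per-tick yaw, so it is frame-rate dependent; SetOrbitLine's logic is disconnected.
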(event EventBeginPlay
  (bind _targetactor (Variables|Default|GetTargetActor))
  (bind _returnvalue (Transformation|GetActorLocation _targetactor))
  ;[1 1 1] Set orbit line preview
  (if (Variables|Default|GetOrbitDraw)
    (bind _returnvalue_2 (Game|SpawnActorfromClass "/Game/SolarSystem/Blueprint/Advanced/Orbit_Blueprint.Orbit_Blueprint_C" (Math|Transform|MakeTransform _returnvalue "0, 0, 0" (/ (Math|Conversions|ToVector(Float) (* (Variables|Default|GetDistance%20from%20Target) 3.0)) 100)) "Undefined" "MultiplyWithRoot" 0 0))
    (Transformation|SetActorLocation _returnvalue_2 _returnvalue false false)
    (Variables|Default|SetInitialLocation (Transformation|GetActorLocation))))

(event EventTick
  (params (DeltaSeconds :type Float%20%28single-precision%29))
  ;[1 1 1] Orbit planet around the sun on each tick
  (Variables|Default|SetCurrentRotation (+ (Variables|Default|GetCurrentRotation) (* (* (Variables|Default|GetOrbit%20Speed) DeltaSeconds) (Math|Float|SelectFloat 1.0 -1.0 (Variables|Default|GetClockwise)))))
  (CallFunction|RotateAroundPoint self (Variables|Default|GetTargetActor) (Variables|Default|GetInitialLocation) (* (Variables|Default|GetDistance%20from%20Target) 3.0) (Variables|Default|GetStartingAngle) (Variables|Default|GetCurrentRotation))
  ;[1 1 1] Own rotation
  (Transformation|AddActorLocalRotation (Math|Rotator|MakeRotator 0.0 0.0 (Variables|Default|GetOwn%20rotation%20speed)) false false))

(fn ConstructionScript)

(fn RotateAroundPoint
  (params (ActorToRotate :type Actor%20Object%20Reference) (ActorTarget :type Actor%20Object%20Reference) (TargetLocation :type Vector) (Radius :type Float%20%28double-precision%29) (Angle :type Float%20%28double-precision%29) (Rotation :type Float%20%28double-precision%29))
  (LocalVariables|SetLocalActorToRotate ActorToRotate)
  (LocalVariables|SetLocalActorTarget ActorTarget)
  (LocalVariables|SetLocalTargetLocation TargetLocation)
  (LocalVariables|SetLocalRadius Radius)
  (LocalVariables|SetLocalAngle Angle)
  (LocalVariables|SetLocalRateOfRotation Rotation)
  (Utilities|IsValid (LocalVariables|GetLocalActorTarget)
    (:Is%20Valid
      (LocalVariables|SetLocalTargetLocation (Transformation|GetActorLocation (LocalVariables|GetLocalActorTarget))))
    (:Is%20Not%20Valid
      _))
  (Transformation|SetActorLocation (LocalVariables|GetLocalActorToRotate) (+ (LocalVariables|GetLocalTargetLocation) (Math|Vector|RotateVectorAroundAxis (Math|Vector|MakeVector (LocalVariables|GetLocalRadius) 0.0 0.0) (+ (LocalVariables|GetLocalAngle) (LocalVariables|GetLocalRateOfRotation)) "0,0.000000,1.000000")) false false)
  (return "0, 0, 0"))

(fn SetOrbitLine
  (params (ActorTarget :type Actor%20Object%20Reference) (TargetLocation :type Vector) (Radius :type Float%20%28double-precision%29) (Angle :type Float%20%28double-precision%29) (RateOfRotation :type Float%20%28double-precision%29)))