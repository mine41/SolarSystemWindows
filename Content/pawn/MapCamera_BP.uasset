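; Map camera pawn that pans, orbits and zooms around a MapOrigin_BP pivot actor found in the level at BeginPlay.
; Enhanced Input look rotates the pivot in fixed steps (local pitch, world yaw), and move input offsets it relative to its yaw.
; Zoom moves the pawn along the pivot-to-pawn line, while Tick keeps the camera aimed at the pivot.
; Helper functions limit pitch, pan area and zoom distance.
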(event Input|EnhancedActionEvents|EnhancedInputActionmy_IA_Look
  (params (ActionValue :type Vector%202D%20Structure) (ElapsedSeconds :type Float%20%28double-precision%29) (TriggeredSeconds :type Float%20%28double-precision%29) (InputAction :type Input%20Action%20Object%20Reference :default "/Game/Input/my_IA_Look.my_IA_Look"))
  (bind _v_rotation_camera (Variables|Default|GetV_rotation_camera))
  (bind _returnvalue (* -1.0 _v_rotation_camera))
  ;[1 1 1] 鼠标控制相机角度
  (:Triggered
    (Utilities|FlowControl|Sequence
      (:then_0
        (if (> (.x ActionValue) 1.0)
          (Development|PrintString "←")
          (Variables|Default|SetRotation_Z _returnvalue)
          (bind _true (CallFunction|InLimitRotationY (Variables|Default|GetMapOrigin) (Variables|Default|GetRotation_Y) :!label _label))
          (if _true
            (Transformation|AddActorLocalRotation (Variables|Default|GetMapOrigin) (Math|Rotator|MakeRotator 0.0 (Variables|Default|GetRotation_Y) 0.0) false false)
            (Class|Actor|AddActorWorldRotation (Variables|Default|GetMapOrigin) (Math|Rotator|MakeRotator 0.0 0.0 (Variables|Default|GetRotation_Z))))
          (elif (< (.x ActionValue) -1.0)
            (Development|PrintString "→")
            (Variables|Default|SetRotation_Z _v_rotation_camera)
            (goto _label))))
      (:then_1
        (if (> (.y ActionValue) 1.0)
          (Development|PrintString "↓")
          (Variables|Default|SetRotation_Y _returnvalue)
          (goto _label)
          (elif (< (.y ActionValue) -1.0)
            (Development|PrintString "↑")
            (Variables|Default|SetRotation_Y _v_rotation_camera)
            (goto _label))))))
  (:Completed
    (Development|PrintString "结束了")
    (Variables|Default|SetRotation_Z 0.0)
    (Variables|Default|SetRotation_Y 0.0)))

(event Input|EnhancedActionEvents|EnhancedInputActionIA_map_move
  (params (ActionValue :type Vector%202D%20Structure) (ElapsedSeconds :type Float%20%28double-precision%29) (TriggeredSeconds :type Float%20%28double-precision%29) (InputAction :type Input%20Action%20Object%20Reference :default "/Game/Input/IA_map_move.IA_map_move"))
  (bind _v_move_origin (Variables|Default|GetV_move_origin))
  (bind _maporigin (Variables|Default|GetMapOrigin))
  (bind _maporigin_2 (Variables|Default|GetMapOrigin))
  (bind _returnvalue (Transformation|GetActorRotation _maporigin))
  (bind _yaw (Math|Rotator|BreakRotator _returnvalue))
  (bind _returnvalue_2 (Math|Trig|Cos(Degrees) _yaw))
  (bind _returnvalue_3 (Math|Trig|Sin(Degrees) _yaw))
  ;[1 1 1] WASD控制移动
  (:Triggered
    (bind _output_get (Variables|Default|SetMoveX (* _v_move_origin (.x ActionValue))))
    (bind _output_get_2 (Variables|Default|SetMoveY (* _v_move_origin (.y ActionValue))))
    (bind _newparam (CallFunction|InLimitLocation (+ (* _output_get _returnvalue_2) (* _returnvalue_3 _output_get_2 -1.0)) (+ (* _output_get _returnvalue_3) (* _returnvalue_2 _output_get_2)) _maporigin_2 (Variables|Default|GetLimit_Location)))
    (if _newparam
      (Transformation|AddActorWorldOffset _maporigin_2 (Math|Vector|MakeVector (+ (* _output_get _returnvalue_2) (* _returnvalue_3 _output_get_2 -1.0)) (+ (* _output_get _returnvalue_3) (* _returnvalue_2 _output_get_2)) 0.0))))
  (:Completed
    (Variables|Default|SetMoveX 0.0)
    (Variables|Default|SetMoveY 0.0)))

(event Input|EnhancedActionEvents|EnhancedInputActionIA_map_updown
  (params (ActionValue :type Float%20%28double-precision%29) (ElapsedSeconds :type Float%20%28double-precision%29) (TriggeredSeconds :type Float%20%28double-precision%29) (InputAction :type Input%20Action%20Object%20Reference :default "/Game/Input/IA_map_updown.IA_map_updown"))
  ;[1 1 1] 相机远近
  (bind _newparam (CallFunction|InLimitHeight (Variables|Default|GetLimit_height) (Variables|Default|GetMapOrigin) ActionValue))
  (if _newparam
    (Transformation|AddActorWorldOffset (* (Math|Vector|Normalize (- (Transformation|GetActorLocation) (Transformation|GetActorLocation (Variables|Default|GetMapOrigin)))) ActionValue (Variables|Default|GetV_move_origin)))))

(event EventBeginPlay
  ;[1 1 1] 初始化地图原点，设置初始相机位置
  (Input|AddMappingContext (PlayerController|LocalPlayerSubsystems|GetEnhancedInputLocalPlayerSubsystem (Game|GetPlayerController 0)) "/Game/Input/my_IMC_default.my_IMC_default" 0 "(bIgnoreAllPressedKeysUntilRelease=True,bForceImmediately=False,bNotifyUserSettings=False)")
  (bind _outactors (Actor|GetAllActorsOfClass "/Game/pawn/MapOrigin_BP.MapOrigin_BP_C"))
  (Variables|Default|SetMapOrigin (Utilities|Array|Get(acopy) _outactors))
  (Transformation|SetActorRelativeLocation (Math|Vector|MakeVector 0.0 0.0 (Variables|Default|GetRadius))))

(event EventTick
  (params (DeltaSeconds :type Float%20%28single-precision%29))
  ;[1 1 1] 相机始终朝向原点
  (Transformation|SetWorldRotation (Variables|Default|GetCamera) (Math|Rotator|FindLookatRotation (Transformation|GetWorldLocation (Variables|Default|GetCamera)) (Transformation|GetActorLocation (Variables|Default|GetMapOrigin))) false false))

(fn ConstructionScript)

(fn InLimitRotationY
  (params (Origin :type Actor%20Object%20Reference) (Rotation_Y :type Float%20%28double-precision%29))
  (bind _returnvalue (Transformation|GetActorRotation Origin))
  (bind _pitch (Math|Rotator|BreakRotator _returnvalue))
  (return (or (and (<= _pitch 6e+01) (>= Rotation_Y 0.0)) (and (<= Rotation_Y 0.0) (>= _pitch 0.0)))))

(fn InLimitLocation
  (params (MoveX :type Float%20%28double-precision%29) (MoveY :type Float%20%28double-precision%29) (Origin :type Actor%20Object%20Reference) (Limit_Location :type Float%20%28double-precision%29))
  (bind _returnvalue (Transformation|GetActorLocation Origin))
  (bind (_x _y) (Math|Vector|BreakVector _returnvalue))
  (return (not (Math|Boolean|ORBoolean (and (>= _x Limit_Location) (> MoveX 0.0)) (and (<= _x (* Limit_Location -1.0)) (< MoveX 0.0)) (and (>= _y Limit_Location) (> MoveY 0.0)) (and (<= _y (* Limit_Location -1.0)) (< MoveY 0.0))))))

(fn InLimitHeight
  (params (Limit_height :type Vector%202D%20Structure) (Origin :type Actor%20Object%20Reference) (ActionValue :type Float%20%28double-precision%29))
  (bind _returnvalue (Transformation|GetActorLocation))
  (bind _returnvalue_2 (Transformation|GetActorLocation Origin))
  (bind _returnvalue_3 (- _returnvalue_2 _returnvalue))
  (bind _returnvalue_4 (Math|Vector|VectorLength _returnvalue_3))
  (return (not (or (and (<= _returnvalue_4 (.x Limit_height)) (< ActionValue 0.0)) (and (>= _returnvalue_4 (.y Limit_height)) (> ActionValue 0.0))))))